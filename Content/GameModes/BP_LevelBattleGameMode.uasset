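; Game mode for a wave-based survival battle level, handling music, tutorials, victory and player death.
; It restores the wave count from the game instance and stores it again before each new wave spawns.
; State changes open data-table tutorials on two waves, save and show an async-loaded demo win screen, or reload the level on death.
; Helper functions create wave text widgets with or without countdowns.
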(event Custom|OnSurvivalGameModeStateChanged_Event
  (params (CurrentState :type EPanWarSurvivalGameModeState%20Enum :default "WaitSpawnNewWave"))
  (switch Utilities|FlowControl|Switch|SwitchonEPanWarSurvivalGameModeState CurrentState
    (:WaitSpawnNewWave
      (Class|PanWarGameInstance|SetCurrentLevelBattleWaveCount (Variables|Default|GetGameInstance) (Variables|Default|GetCurrentWaveCount))
      (switch int (Variables|Default|GetCurrentWaveCount)
        (:2
          (Variables|Default|SetTutorial%20Row%20Name "Block"))
        (:5
          (Variables|Default|SetTutorial%20Row%20Name "UnblockableAttack")))
      (CallFunction|OpenTutorial))
    (:AllWavesDone
      (Utilities|FlowControl|Delay 1.5)
      (Viewport|RemoveAllWidgets)
      (CameraFades|StartCameraFade :self (Game|GetPlayerCameraManager 0) :ToAlpha 1.0 :Duration 3.0 :bHoldWhenFinished true)
      (Audio|Components|Audio|Stop (stale EventBeginPlay _returnvalue))
      (Audio|SpawnSound2D "/Game/Fantasy_Starter_Pack/WAVs/The_Warrior_Cave_Troll_Full.The_Warrior_Cave_Troll_Full" 0.7 1.0 0.0 0)
      (Utilities|FlowControl|Delay 3.0)
      (Class|PanWarFunctionLibrary|SaveCurrentGameLevel "Level_1")
      (bind _class (Utilities|AsyncLoadClassAsset "/Game/UI/Widgets/GameModeWidgets/WBP_WinDemoScreen.WBP_WinDemoScreen_C")
        (:Completed
          (bind _asuser_widget (Utilities|Casting|CastToUserWidgetClass _class))
          (bind _returnvalue (UserInterface|CreateWidget _asuser_widget))
          (UserInterface|Viewport|AddtoViewport _returnvalue 0))))
    (:PlayerDied
      (Viewport|RemoveAllWidgets)
      (CameraFades|StartCameraFade :self (Game|GetPlayerCameraManager 0) :ToAlpha 1.0 :Duration 2.0 :bHoldWhenFinished true)
      (Utilities|FlowControl|Delay 2.0)
      (bind _outactors (Actor|GetAllActorsOfClass "/Script/PanWolfWar.BaseEnemy"))
      (for _array_element _outactors
        (Actor|DestroyActor _array_element))
      (bind _returnvalue_2 (Game|GetCurrentLevelName true))
      (Game|OpenLevel(byName) (Utilities|String|StringToName _returnvalue_2))
      (Class|PanWarFunctionLibrary|ToggleInputMode "GameOnly"))))

(event EventBeginPlay
  (bind _returnvalue (Audio|SpawnSound2D "/Game/Fantasy_Starter_Pack/WAVs/The_Warrior_Regroup_Full.The_Warrior_Regroup_Full" 0.7 1.0 0.0 0))
  (EventDispatchers|AssignOnSurvivalGameModeStateChanged (delegate Custom|OnSurvivalGameModeStateChanged_Event))
  (Variables|Default|SetGameInstance (Class|PanWarFunctionLibrary|GetPanWarGameInstance))
  (Class|PanWarSurvivalGameMode|SetCurrentWaveCount (Class|PanWarGameInstance|GetCurrentLevelBattleWaveCount (Variables|Default|GetGameInstance))))

(fn ConstructionScript)

(fn CreateWaveWidgetwithCountDown
  (params (TextContentToDisplay :type Text) (InTotalCountDownTime :type Float%20%28double-precision%29))
  (bind _returnvalue (UserInterface|CreateWidget "/Game/UI/Widgets/GameModeWidgets/WBP_WaveTextWithCountDown.WBP_WaveTextWithCountDown_C"))
  (UserInterface|Viewport|AddtoViewport _returnvalue 0)
  (Rendering|Components|TextRender|SetText (Variables|/Game/UI/Widgets/GameModeWidgets/WBP_WaveTextWithCountDown.WBP_WaveTextWithCountDown_C|GetTextBlock_WaveText _returnvalue) TextContentToDisplay)
  (Default|StartCountDown _returnvalue InTotalCountDownTime))

(fn CreateWaveWidgetNoCountDown
  (params (TextContentToDisplay :type Text))
  (bind _returnvalue (UserInterface|CreateWidget "/Game/UI/Widgets/GameModeWidgets/WBP_WaveTextNoCountDown.WBP_WaveTextNoCountDown_C"))
  (UserInterface|Viewport|AddtoViewport _returnvalue 0)
  (Rendering|Components|TextRender|SetText (Variables|/Game/UI/Widgets/GameModeWidgets/WBP_WaveTextNoCountDown.WBP_WaveTextNoCountDown_C|GetTextBlock_WaveText _returnvalue) TextContentToDisplay))

(fn OpenTutorial
  (bind _aspan_war_game_instance (Utilities|Casting|CastToPanWarGameInstance (Game|GetGameInstance)))
  (bind _returnvalue (Utilities|GetDataTableRow (Variables|/Script/PanWolfWar.PanWarGameInstance|GetTutorialDataTable _aspan_war_game_instance) (Variables|Default|GetTutorial%20Row%20Name))
    (:then
      (bind _returnvalue_2 (UserInterface|CreateWidget "/Game/UI/Widgets/TutorialWidgets/WBP_TutorialWidget.WBP_TutorialWidget_C" 0 (.TutorialValues (Utilities|Struct|BreakTutorialContainer _returnvalue))))
      (UserInterface|Viewport|AddtoViewport _returnvalue_2 0))))