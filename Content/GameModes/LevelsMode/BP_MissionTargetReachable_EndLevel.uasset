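; Mission target that ends the level when reached and loads the next one.
; When the mission activates, its box component begins overlapping Pawn and PhysicsBody channels.
; On the target-reached event, it starts a held camera fade-out, then opens the NextLevel reference after a short delay that ends before the fade completes.
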(event EventBeginPlay
  (|CallParentFunction) ; This node is disabled and will not be called.\nDrag off pins to build functionality.
)

(event Collision|EventActorBeginOverlap
  (params (OtherActor :type Actor%20Object%20Reference))
  (|CallParentFunction OtherActor) ; This node is disabled and will not be called.\nDrag off pins to build functionality.
)

(event EventTick
  (params (DeltaSeconds :type Float%20%28single-precision%29))
  (|CallParentFunction DeltaSeconds) ; This node is disabled and will not be called.\nDrag off pins to build functionality.
)

(event EventOnTargetReached
  (CameraFades|StartCameraFade :self (Game|GetPlayerCameraManager 0) :ToAlpha 1.0 :Duration 3.0 :bHoldWhenFinished true)
  (Utilities|FlowControl|Delay 1.0)
  (Game|OpenLevel(byObjectReference) (Variables|Default|GetNextLevel)))

(event EventOnTargetMissionActivated
  (Collision|SetCollisionResponsetoChannel (Variables|Default|GetBoxComponent) "ECC_Pawn" "ECR_Overlap")
  (Collision|SetCollisionResponsetoChannel (Variables|Default|GetBoxComponent) "ECC_PhysicsBody" "ECR_Overlap"))

(fn ConstructionScript
  (|CallParentFunction))