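; A mission target fog wall for the levels game mode, built around a FogCube component that can be shown or cleared.
; When the target mission activates, the cube is hidden and its collision is disabled.
; The ActivateFog event reverses this, making the cube visible with query and physics collision.
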(event Custom|ActivateFog
  (bind _fogcube (Variables|Default|GetFogCube))
  (Collision|SetCollisionEnabled _fogcube "QueryAndPhysics")
  (Rendering|SetVisibility _fogcube true false))

(event EventBeginPlay
  (|CallParentFunction) ; This node is disabled and will not be called.\nDrag off pins to build functionality.
)

(event Collision|EventActorBeginOverlap
  (params (OtherActor :type Actor%20Object%20Reference))
  (|CallParentFunction OtherActor) ; This node is disabled and will not be called.\nDrag off pins to build functionality.
)

(event EventTick
  (params (DeltaSeconds :type Float%20%28single-precision%29))
  (|CallParentFunction DeltaSeconds) ; This node is disabled and will not be called.\nDrag off pins to build functionality.
)

(event EventOnTargetMissionActivated
  (bind _fogcube (Variables|Default|GetFogCube))
  (Collision|SetCollisionEnabled _fogcube "NoCollision")
  (Rendering|SetVisibility _fogcube false false))

(fn ConstructionScript
  (|CallParentFunction))