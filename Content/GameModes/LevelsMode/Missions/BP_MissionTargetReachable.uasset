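; BP_MissionTargetReachable is a levels-mode mission target that triggers optional follow-up events when the target is reached.
; On reach, it can activate fog on a referenced FogTarget and, separately, start a battle, each gated by its own flag.
; Starting battle sets the BP_LevelBattleGameMode survival state to spawning a new wave and puts the player's PanWolfWarCharacter into battle mode.
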(event EventOnTargetReached
  (Utilities|FlowControl|Sequence
    (:then_0
      (if (Variables|Default|GetIsActivateFog)
        (bind _fogtarget (Variables|Default|GetFogTarget)
          (:then
            (Default|ActivateFog _fogtarget))
          (:else))))
    (:then_1
      (if (Variables|Default|GetIsActivateBattle)
        (bind _asbp_level_battle_game_mode (Utilities|Casting|CastToBP_LevelBattleGameMode (Game|GetGameMode)))
        (Class|PanWarSurvivalGameMode|SetCurrentSurvivalGameModeState _asbp_level_battle_game_mode "SpawningNewWave")
        (bind _aspan_wolf_war_character (Utilities|Casting|CastToPanWolfWarCharacter (Game|GetPlayerCharacter 0)))
        (Class|PanWolfWarCharacter|EnterBattleMode _aspan_wolf_war_character)))))

(fn ConstructionScript)