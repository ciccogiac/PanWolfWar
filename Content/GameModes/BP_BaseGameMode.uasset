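; Base game mode that handles player death by restarting the current level.
; Its PlayerDie event clears all widgets and fades the camera out, holding the faded screen.
; After a delay matching the fade, it destroys every BaseEnemy actor, reopens the current level by name and switches input to game-only.
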(event EventPlayerDie
  (Viewport|RemoveAllWidgets)
  (CameraFades|StartCameraFade :self (Game|GetPlayerCameraManager 0) :ToAlpha 1.0 :Duration 2.0 :bHoldWhenFinished true)
  (Utilities|FlowControl|Delay 2.0)
  (bind _outactors (Actor|GetAllActorsOfClass "/Script/PanWolfWar.BaseEnemy"))
  (for _array_element _outactors
    (Actor|DestroyActor _array_element))
  (bind _returnvalue (Game|GetCurrentLevelName true))
  (Game|OpenLevel(byName) (Utilities|String|StringToName _returnvalue))
  (Class|PanWarFunctionLibrary|ToggleInputMode "GameOnly"))

(fn ConstructionScript)