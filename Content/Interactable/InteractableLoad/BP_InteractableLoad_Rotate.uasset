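; BP_InteractableLoad_Rotate is an interactable that rotates and shifts its static mesh according to the progress value passed to its Interaction event.
; BeginPlay caches the mesh's relative location as the base position.
; Interaction samples three float curves at Percent: one sets pitch, with roll and yaw held at zero, and two add X and Z offsets to that base, so curve data shapes the whole motion.
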(event EventBeginPlay
  (|CallParentFunction)
  (Variables|Default|SetNewVar_0 (Variables|/Script/Engine.SceneComponent|GetRelativeLocation (Variables|Default|GetStaticMesh))))

(event Collision|EventActorBeginOverlap
  (params (OtherActor :type Actor%20Object%20Reference))
  (|CallParentFunction OtherActor) ; This node is disabled and will not be called.\nDrag off pins to build functionality.
)

(event EventTick
  (params (DeltaSeconds :type Float%20%28single-precision%29))
  (|CallParentFunction DeltaSeconds) ; This node is disabled and will not be called.\nDrag off pins to build functionality.
)

(event EventInteraction
  (params (Percent :type Float%20%28single-precision%29))
  (bind _staticmesh (Variables|Default|GetStaticMesh))
  (Transformation|SetRelativeRotation _staticmesh (Math|Rotator|MakeRotator 0.0 (Math|Curves|GetFloatValue (Variables|Default|Getcurve) Percent) 0.0) false false)
  (Transformation|SetRelativeLocation _staticmesh (+ (Variables|Default|GetNewVar_0) (Math|Vector|MakeVector (Math|Curves|GetFloatValue (Variables|Default|Getcurve_0) Percent) 0.0 (Math|Curves|GetFloatValue (Variables|Default|Getcurve_1) Percent))) false false))

(fn ConstructionScript
  (|CallParentFunction))