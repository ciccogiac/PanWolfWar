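; BP_InteractableLoad_Move is an interactable that rotates its static mesh in response to interaction.
; On each Interaction event, it adds the incoming Percent value directly to the mesh's local pitch as degrees, so rotation accumulates across calls.
; BeginPlay and construction only call the parent, and the Blueprint has no active Tick or overlap logic of its own.
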(event EventBeginPlay
  (|CallParentFunction))

(event Collision|EventActorBeginOverlap
  (params (OtherActor :type Actor%20Object%20Reference))
  (|CallParentFunction OtherActor) ; This node is disabled and will not be called.\nDrag off pins to build functionality.
)

(event EventTick
  (params (DeltaSeconds :type Float%20%28single-precision%29))
  (|CallParentFunction DeltaSeconds) ; This node is disabled and will not be called.\nDrag off pins to build functionality.
)

(event EventInteraction
  (params (Percent :type Float%20%28single-precision%29))
  (Transformation|AddLocalRotation (Variables|Default|GetStaticMesh) (Math|Rotator|MakeRotator 0.0 Percent 0.0) false false))

(fn ConstructionScript
  (|CallParentFunction))