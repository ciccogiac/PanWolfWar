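; Player character Blueprint for Pando, adding kite controls, the pause menu and developer debug keys.
; Kite input drives a Timeline that tilts the attached BP_Kite mesh and reverses on release, while exit calls LeavKite on Molo.
; Debug keys toggle component traces and climbable box visibility, self-damage, reload checkpoints and toggle slow motion.
; Pause async-loads its widget class; several state-print and kite-rotation chains are left unconnected.
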(event Input|EnhancedActionEvents|EnhancedInputActionIA_KiteExit
  (params (ActionValue :type Boolean) (ElapsedSeconds :type Float%20%28double-precision%29) (TriggeredSeconds :type Float%20%28double-precision%29) (InputAction :type Input%20Action%20Object%20Reference :default "/Game/Transformation/Pandolfo/Kite/Input/IA_KiteExit.IA_KiteExit"))
  ;[1 1 1] Kite
  (:Completed
    (bind _molo (Variables|Default|GetMolo)
      (:then
        (Default|LeavKite _molo))
      (:else))))

(event Input|EnhancedActionEvents|EnhancedInputActionIA_KiteMove
  (params (ActionValue :type Vector%202D%20Structure) (ElapsedSeconds :type Float%20%28double-precision%29) (TriggeredSeconds :type Float%20%28double-precision%29) (InputAction :type Input%20Action%20Object%20Reference :default "/Game/Transformation/Pandolfo/Kite/Input/IA_KiteMove.IA_KiteMove"))
  ;[1 1 1] Kite
  (:Triggered
    (bind _returnvalue (Actor|GetActorOfClass "/Game/Transformation/Pandolfo/Kite/Kite/BP_Kite.BP_Kite_C"))
    (if (Variables|/Game/Transformation/Pandolfo/Kite/Kite/BP_Kite.BP_Kite_C|GetIsAttached _returnvalue)
      (if (> (.Y (Math|Vector2D|BreakVector2D ActionValue)) 0.0)
        (bind (_direction _newtrack_0 _newtrack_1) (Timeline|Timeline Play)
          (:Update
            (Transformation|SetRelativeRotation (Variables|/Game/Transformation/Pandolfo/Kite/Kite/BP_Kite.BP_Kite_C|GetStaticMesh _returnvalue) (Math|Rotator|MakeRotator _newtrack_1 1.8e+02 _newtrack_0) false false))))))
  (:Completed
    (Timeline|Timeline Reverse)))

(event Input|EnhancedActionEvents|EnhancedInputActionIA_PauseMenu
  (params (ActionValue :type Boolean) (ElapsedSeconds :type Float%20%28double-precision%29) (TriggeredSeconds :type Float%20%28double-precision%29) (InputAction :type Input%20Action%20Object%20Reference :default "/Game/ThirdPerson/Input/Actions/IA_PauseMenu.IA_PauseMenu"))
  ;[1 1 1] Pause
  (:Started
    (bind _class (Utilities|AsyncLoadClassAsset "/Game/UI/Widgets/GameModeWidgets/WBP_PauseScreen.WBP_PauseScreen_C")
      (:Completed
        (bind _asuser_widget (Utilities|Casting|CastToUserWidgetClass _class))
        (bind _returnvalue (UserInterface|CreateWidget _asuser_widget))
        (UserInterface|Viewport|AddtoViewport _returnvalue 0)))))

(event EventBeginPlay
  (bind _outactors (Actor|GetAllActorsOfClass "/Game/Climbing/ClimbableObjects/ClimbableBOX.ClimbableBOX_C"))
  (Variables|Default|SetAllCLimbables _outactors))

(event EventTick
  (params (DeltaSeconds :type Float%20%28single-precision%29)))

(event Input|KeyboardEvents|DebugKey1
  (params (Key :type Key%20Structure :default "None") (ActionValue :type Input%20Action%20Value%20Structure))
  (bind _pandolfocomponent (Variables|Default|GetPandolfoComponent))
  (bind _climbingcomponent (Variables|/Script/PanWolfWar.PandolfoComponent|GetClimbingComponent _pandolfocomponent))
  ;[1 1 1] Enable Climbing Debug Show
  (:Pressed
    (Variables|/Script/PanWolfWar.ClimbingComponent|SetShowDebugTrace _climbingcomponent (not (Variables|/Script/PanWolfWar.ClimbingComponent|GetShowDebugTrace _climbingcomponent)))
    (for _array_element (Variables|Default|GetAllCLimbables)
      (Rendering|SetActorHiddenInGame _array_element (not (Variables|/Script/PanWolfWar.ClimbingComponent|GetShowDebugTrace _climbingcomponent))))
    (if (not (Variables|/Script/PanWolfWar.ClimbingComponent|GetShowDebugTrace _climbingcomponent))
      (Development|PrintString "Debug Trace Disabled" true true "(R=1.000000,G=0.000000,B=0.390800,A=1.000000)" 5.0 "10")
      (else
        (Development|PrintString "Debug Trace Enabled" true true "(R=1.000000,G=0.000000,B=0.390800,A=1.000000)" 5.0 "10")))))

(event Input|KeyboardEvents|DebugKey2
  (params (Key :type Key%20Structure :default "None") (ActionValue :type Input%20Action%20Value%20Structure))
  (bind _pandolflowercomponent (Variables|Default|GetPandolFlowerComponent))
  ;[1 1 1] Enable Climbing Debug Show
  (:Pressed
    (Variables|/Script/PanWolfWar.PandolFlowerComponent|SetShowDebugTrace _pandolflowercomponent (not (Variables|/Script/PanWolfWar.PandolFlowerComponent|GetShowDebugTrace _pandolflowercomponent)))))

(event Input|KeyboardEvents|DebugKey3
  (params (Key :type Key%20Structure :default "None") (ActionValue :type Input%20Action%20Value%20Structure))
  (bind _pandolfocomponent (Variables|Default|GetPandolfoComponent))
  (bind _sneakcovercomponent (Variables|/Script/PanWolfWar.PandolfoComponent|GetSneakCoverComponent _pandolfocomponent))
  ;[1 1 1] Enable Climbing Debug Show
  (:Pressed
    (Variables|/Script/PanWolfWar.SneakCoverComponent|SetShowDebugTrace _sneakcovercomponent (not (Variables|/Script/PanWolfWar.SneakCoverComponent|GetShowDebugTrace _sneakcovercomponent)))))

(event Input|KeyboardEvents|DebugKey4
  (params (Key :type Key%20Structure :default "None") (ActionValue :type Input%20Action%20Value%20Structure))
  (bind _pandolfocomponent (Variables|Default|GetPandolfoComponent))
  ;[1 1 1] Enable Climbing Debug Show
  (:Pressed
    (Variables|/Script/PanWolfWar.PandolfoComponent|SetShowDebugTrace _pandolfocomponent (not (Variables|/Script/PanWolfWar.PandolfoComponent|GetShowDebugTrace _pandolfocomponent)))))

(event Input|KeyboardEvents|DebugKeyP
  (params (Key :type Key%20Structure :default "None") (ActionValue :type Input%20Action%20Value%20Structure))
  (:Pressed
    (bind _asclimbing_game_mode (Utilities|Casting|CastToClimbing_GameMode (Game|GetGameMode)))
    (Default|ReloadCheckPoint _asclimbing_game_mode)))

(event Input|KeyboardEvents|DebugKeyQ
  (params (Key :type Key%20Structure :default "None") (ActionValue :type Input%20Action%20Value%20Structure))
  ;[0.02604 0.02604 0.02604] Slow Motion
  (:Pressed
    (Utilities|FlowControl|FlipFlop
      (:A
        (Utilities|Time|SetGlobalTimeDilation 0.2))
      (:B
        (Utilities|Time|SetGlobalTimeDilation 1.0)))))

(event Input|KeyboardEvents|DebugKey5
  (params (Key :type Key%20Structure :default "None") (ActionValue :type Input%20Action%20Value%20Structure))
  (bind _pandocombatcomponent (Variables|Default|GetPandoCombatComponent))
  ;[1 1 1] Enable Climbing Debug Show
  (:Pressed
    (bind _output_get (Variables|/Script/PanWolfWar.PawnCombatComponent|SetShowDebugTrace _pandocombatcomponent (not (Variables|/Script/PanWolfWar.PawnCombatComponent|GetShowDebugTrace _pandocombatcomponent))))
    (if _output_get
      (Development|PrintString "Combat Debug Trace Enabled" true true "(R=1.000000,G=0.000000,B=0.390800,A=1.000000)" 5.0 "10")
      (else
        (Development|PrintString "Combat Debug Trace Disabled" true true "(R=1.000000,G=0.000000,B=0.390800,A=1.000000)" 5.0 "10")))))

(event Input|KeyboardEvents|DebugKey9
  (params (Key :type Key%20Structure :default "None") (ActionValue :type Input%20Action%20Value%20Structure))
  (bind _self self)
  (:Pressed
    (Game|Damage|ApplyDamage _self 5.0 (Pawn|GetController (Game|GetInstigator _self)) _self "/Script/Engine.DamageType")
    (Class|HitInterface|GetHit (Transformation|GetActorLocation) _self)))

(fn ConstructionScript)