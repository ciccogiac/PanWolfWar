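; BP_Hide is a stealth hiding zone for the PanWolfWar player character.
; On BeginPlay it finds and caches the PanWolfWarCharacter in the level.
; Its Box overlap events turn that character's hiding state on when it enters and off when it leaves, with the crouch check enabled both times.
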(event OnComponentBeginOverlap(Box)
  (params (OverlappedComponent :type Primitive%20Component%20Object%20Reference) (OtherActor :type Actor%20Object%20Reference) (OtherComp :type Primitive%20Component%20Object%20Reference) (OtherBodyIndex :type Integer) (bFromSweep :type Boolean) (SweepResult :type Hit%20Result%20Structure%20%28by%20ref%29))
  (if (== (Variables|Default|GetPan%20Wolf%20War%20Character) OtherActor)
    (Class|PanWolfWarCharacter|SetIsHiding (Variables|Default|GetPan%20Wolf%20War%20Character) true true)))

(event OnComponentEndOverlap(Box)
  (params (OverlappedComponent :type Primitive%20Component%20Object%20Reference) (OtherActor :type Actor%20Object%20Reference) (OtherComp :type Primitive%20Component%20Object%20Reference) (OtherBodyIndex :type Integer))
  (if (== (Variables|Default|GetPan%20Wolf%20War%20Character) OtherActor)
    (Class|PanWolfWarCharacter|SetIsHiding (Variables|Default|GetPan%20Wolf%20War%20Character) false true)))

(event EventBeginPlay
  (bind _returnvalue (Actor|GetActorOfClass "/Script/PanWolfWar.PanWolfWarCharacter"))
  (Variables|Default|SetPan%20Wolf%20War%20Character _returnvalue))

(event Collision|EventActorBeginOverlap
  (params (OtherActor :type Actor%20Object%20Reference)))

(event EventTick
  (params (DeltaSeconds :type Float%20%28single-precision%29)))

(fn ConstructionScript)