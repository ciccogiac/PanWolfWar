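; BP_Kite is a kite actor that attaches to and detaches from the Pando character.
; AttachKite finds BP_PandoCharacter by class, snaps the kite to its mesh with the bar mesh on KiteBar_Socket, and corrects mesh rotations.
; It also shifts the character's camera boom back and up.
; DetachKite clears IsAttached and detaches in place, without restoring the camera offset.
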(event Custom|DetachKite
  (Variables|Default|SetIsAttached false)
  (Transformation|DetachFromActor "KeepWorld" "KeepWorld" "KeepWorld")
  (Transformation|DetachFromComponent (Variables|Default|GetStaticMesh) "KeepWorld" "KeepWorld" "KeepWorld" true))

(event Custom|AttachKite
  (bind _returnvalue (Actor|GetActorOfClass "/Game/Transformation/BP_PandoCharacter.BP_PandoCharacter_C"))
  (Transformation|AttachComponentToComponent (Variables|/Script/Engine.Character|GetMesh _returnvalue) "None" "SnapToTarget" "SnapToTarget" "KeepWorld" true)
  (Transformation|AttachComponentToComponent (Variables|Default|GetStaticMesh) (Variables|/Script/Engine.Character|GetMesh _returnvalue) "KiteBar_Socket" "SnapToTarget" "SnapToTarget" "KeepWorld" true)
  (Transformation|SetRelativeRotation (Variables|Default|GetStaticMesh) "180.000000,0.000000,180.000000" false false)
  (Transformation|SetRelativeRotation (Variables|Default|GetKiteMesh) "90.000000,180.000000,180.000000" false false)
  (Transformation|AddLocalOffset (Variables|/Script/PanWolfWar.PanWolfWarCharacter|GetCameraBoom _returnvalue) "-200.000000,0.000000,50.000000" false false)
  (Variables|Default|SetIsAttached true))

(fn ConstructionScript)