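; BP_Molo is a kitesurfing exit point where the Pandolfo character can leave kite mode.
; Its box overlap shows a widget and plane and registers itself on the character if the Pandolfo component is active and Kiting, clearing both on exit.
; LeavKite exits kite mode, offsets the camera boom, detaches kite and character, stops board physics and makes the sea ignore the Visibility channel, finding those world actors by class.
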(event OnComponentBeginOverlap(Box)
  (params (OverlappedComponent :type Primitive%20Component%20Object%20Reference) (OtherActor :type Actor%20Object%20Reference) (OtherComp :type Primitive%20Component%20Object%20Reference) (OtherBodyIndex :type Integer) (bFromSweep :type Boolean) (SweepResult :type Hit%20Result%20Structure%20%28by%20ref%29))
  (bind _asbp_pando_character (Utilities|Casting|CastToBP_PandoCharacter OtherActor))
  (if (and (Components|Activation|IsActive (Variables|/Script/PanWolfWar.PanWolfWarCharacter|GetPandolfoComponent _asbp_pando_character)) (Utilities|Enum|Equal(Enum) (Variables|/Script/PanWolfWar.PandolfoComponent|GetPandolfoState (Variables|/Script/PanWolfWar.PanWolfWarCharacter|GetPandolfoComponent _asbp_pando_character)) "EPS_Kiting"))
    (bind _output_get (Variables|Default|SetAs%20BP%20Third%20Person%20Character _asbp_pando_character))
    (Rendering|SetVisibility (Variables|Default|GetWidget) true false)
    (Variables|/Game/Transformation/BP_PandoCharacter.BP_PandoCharacter_C|SetMolo _output_get self)))

(event OnComponentEndOverlap(Box)
  (params (OverlappedComponent :type Primitive%20Component%20Object%20Reference) (OtherActor :type Actor%20Object%20Reference) (OtherComp :type Primitive%20Component%20Object%20Reference) (OtherBodyIndex :type Integer))
  (bind _asbp_pando_character (Utilities|Casting|CastToBP_PandoCharacter OtherActor))
  (Rendering|SetVisibility (Variables|Default|GetWidget) false false)
  (Variables|/Game/Transformation/BP_PandoCharacter.BP_PandoCharacter_C|SetMolo _asbp_pando_character 0))

(event Custom|LeavKite
  (Rendering|SetVisibility (Variables|Default|GetWidget) false false)
  (Class|PandolfoComponent|ExitKiteMode (Variables|/Script/PanWolfWar.PanWolfWarCharacter|GetPandolfoComponent (Variables|Default|GetAs%20BP%20Third%20Person%20Character)))
  (Transformation|AddLocalOffset (Variables|/Script/PanWolfWar.PanWolfWarCharacter|GetCameraBoom (Variables|Default|GetAs%20BP%20Third%20Person%20Character)) "200.000000,0.000000,-50.000000" false false)
  (bind _returnvalue (Actor|GetActorOfClass "/Game/Transformation/Pandolfo/Kite/Kite/BP_Kite.BP_Kite_C"))
  (Default|DetachKite _returnvalue)
  (bind _returnvalue_2 (Actor|GetActorOfClass "/Game/Transformation/Pandolfo/Kite/Board/BP_KiteBoards.BP_KiteBoards_C"))
  (Physics|SetSimulatePhysics (Variables|/Script/PanWolfWar.InteractableObject|GetStaticMesh _returnvalue_2) false)
  (Transformation|DetachFromActor (Variables|Default|GetAs%20BP%20Third%20Person%20Character) "KeepWorld" "KeepWorld" "KeepWorld")
  (bind _returnvalue_3 (Actor|GetActorOfClass "/Game/Transformation/Pandolfo/Kite/Kite/BP_WaterSea.BP_WaterSea_C"))
  (Collision|SetCollisionResponsetoChannel (Variables|/Script/Engine.StaticMeshActor|GetStaticMeshComponent _returnvalue_3) "ECC_Visibility" "ECR_Ignore"))

(event EventBeginPlay)

(event Collision|EventActorBeginOverlap
  (params (OtherActor :type Actor%20Object%20Reference)))

(event EventTick
  (params (DeltaSeconds :type Float%20%28single-precision%29)))

(fn ConstructionScript)