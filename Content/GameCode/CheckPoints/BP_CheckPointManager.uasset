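; Checkpoint manager actor that sets the player's initial position from the saved checkpoint when play begins.
; On BeginPlay it reads CheckPointNumber from BP_GameInstanceProva and uses it to index its CheckPoints array.
; It passes the world transform of that checkpoint's POS component to Climbing_GameMode through SetInitialPosition.
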(event EventBeginPlay
  (bind _asbp_game_instance_prova (Utilities|Casting|CastToBP_GameInstanceProva (Game|GetGameInstance)))
  (Utilities|IsValid _asbp_game_instance_prova
    (:Is%20Valid
      (bind _asclimbing_game_mode (Utilities|Casting|CastToClimbing_GameMode (Game|GetGameMode)))
      (Default|SetInitialPosition _asclimbing_game_mode (Transformation|GetWorldTransform (Variables|/Game/GameCode/CheckPoints/BP_CheckPoint.BP_CheckPoint_C|GetPOS (Utilities|Array|Get(acopy) (Variables|Default|GetCheckPoints) (Variables|/Game/GameCode/BP_GameInstanceProva.BP_GameInstanceProva_C|GetCheckPoint_Number _asbp_game_instance_prova))))))))

(event Collision|EventActorBeginOverlap
  (params (OtherActor :type Actor%20Object%20Reference)))

(event EventTick
  (params (DeltaSeconds :type Float%20%28single-precision%29)))

(fn ConstructionScript)