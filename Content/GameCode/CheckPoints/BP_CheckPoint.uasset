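; BP_CheckPoint is a one-shot checkpoint actor that records the player's progress in the game instance.
; When a BP_PandoCharacter overlaps its Trigger, it compares its CheckPointNumber with the one stored in BP_GameInstanceProva.
; If its number is higher, it overwrites the stored value, marks itself Used and plays a 2D sound, so progress only moves forward.
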(event OnComponentBeginOverlap(Trigger)
  (params (OverlappedComponent :type Primitive%20Component%20Object%20Reference) (OtherActor :type Actor%20Object%20Reference) (OtherComp :type Primitive%20Component%20Object%20Reference) (OtherBodyIndex :type Integer) (bFromSweep :type Boolean) (SweepResult :type Hit%20Result%20Structure%20%28by%20ref%29))
  (if (not (Variables|Default|GetbUsed))
    (Utilities|Casting|CastToBP_PandoCharacter OtherActor)
    (bind _asbp_game_instance_prova (Utilities|Casting|CastToBP_GameInstanceProva (Game|GetGameInstance)))
    (if (< (Variables|/Game/GameCode/BP_GameInstanceProva.BP_GameInstanceProva_C|GetCheckPoint_Number _asbp_game_instance_prova) (Variables|Default|GetCheckPoint_Number))
      (Variables|/Game/GameCode/BP_GameInstanceProva.BP_GameInstanceProva_C|SetCheckPoint_Number _asbp_game_instance_prova (Variables|Default|GetCheckPoint_Number))
      (Variables|Default|SetbUsed true)
      (Audio|PlaySound2D "/Engine/VREditor/Sounds/UI/Dockable_Window_Drop.Dockable_Window_Drop" 1.0 1.0 0.0 0 0))))

(event EventBeginPlay)

(event Collision|EventActorBeginOverlap
  (params (OtherActor :type Actor%20Object%20Reference)))

(event EventTick
  (params (DeltaSeconds :type Float%20%28single-precision%29)))

(fn ConstructionScript)