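; BP_Gruntling_Glacer is the Blueprint for the Glacer Gruntling, a standard enemy with a projectile attack.
; On BeginPlay it spawns its weapon, then runs the parent's BeginPlay.
; FireProjectile plays the Glacer fire montage on the mesh only when the anim instance is valid and no other montage is playing.
; The graph itself spawns no projectile, and the construction script only calls the parent.
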(event EventBeginPlay
  (CallFunction|SpawnWeapon)
  (|CallParentFunction))

(event Collision|EventActorBeginOverlap
  (params (OtherActor :type Actor%20Object%20Reference)))

(event EventTick
  (params (DeltaSeconds :type Float%20%28single-precision%29)))

(event EventFireProjectile
  (bind _mesh (Variables|Character|GetMesh))
  (bind _returnvalue (Components|SkeletalMesh|GetAnimInstance _mesh))
  (Utilities|IsValid _returnvalue
    (:Is%20Valid
      (if (not (Class|AnimInstance|IsAnyMontagePlaying _returnvalue))
        (Animation|Montage|PlayMontage (Variables|Character|GetMesh) "/Game/Enemy/StandardEnemies/Glacer/AM_Glacer_FireProjectile.AM_Glacer_FireProjectile")))))

(fn ConstructionScript
  (|CallParentFunction))