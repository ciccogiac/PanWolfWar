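; Base enemy character Blueprint that handles dissolve-in entry, dissolve-out death, weapon spawning and stone drops.
; BeginPlay reverses a dissolve timeline on mesh and weapon and plays a random entry montage.
; Death async-loads a color-matched Niagara effect, then dissolves both before destroying them.
; Halfway through, if a weapon is equipped, an attribute-driven roll may async-spawn a healing stone at a random nearby navigable point.
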(event EventBeginPlay
  (bind _entrymontagestoplay (Variables|Default|GetEntryMontagesToPlay))
  (bind _enemycombatcomponent (Variables|Default|GetEnemyCombatComponent))
  (bind _returnvalue (Class|PawnCombatComponent|GetCurrentEquippedWeapon _enemycombatcomponent))
  (Utilities|FlowControl|Sequence
    (:then_0
      (Components|Timeline|SetPlayRate (Variables|Default|GetEntryRestoreTimeline) (/ 1.0 (Variables|Default|GetTotalEntryRestoreTime)))
      (bind _normalizedfloattrack (Timeline|EntryRestoreTimeline ReverseFromEnd)
        (:Update
          (Rendering|Material|SetScalarParameterValueonMaterials (Variables|Character|GetMesh) "DissolveAmount" _normalizedfloattrack)
          (Utilities|IsValid _returnvalue
            (:Is%20Valid
              (Rendering|Material|SetScalarParameterValueonMaterials (Variables|/Script/PanWolfWar.PanWarWeaponBase|GetWeaponMesh _returnvalue) "DissolveAmount" _normalizedfloattrack))))))
    (:then_1
      (if (Utilities|Array|IsNotEmpty _entrymontagestoplay)
        (Animation|PlayAnimMontage (.OutItem (Utilities|Array|Random _entrymontagestoplay)) 1.0 "None")))))

(event EventOnEnemyDieEvent
  (bind _enemycombatcomponent (Variables|Default|GetEnemyCombatComponent))
  (bind _enemycombatcomponent_2 (Variables|Default|GetEnemyCombatComponent))
  (bind _mesh (Variables|Character|GetMesh))
  (bind _dissolveniagarasystem (Variables|Default|GetDissolveNiagaraSystem))
  (bind _returnvalue (Class|PawnCombatComponent|GetCurrentEquippedWeapon _enemycombatcomponent))
  (bind _returnvalue_2 (Class|PawnCombatComponent|GetCurrentEquippedWeapon _enemycombatcomponent_2))
  (if (Utilities|IsValidSoftObjectReference _dissolveniagarasystem)
    (bind _object (Utilities|AsyncLoadAsset _dissolveniagarasystem)
      (:Completed
        (bind _asniagara_system (Utilities|Casting|CastToNiagaraSystem _object))
        (bind _returnvalue_3 (Niagara|SpawnSystemAttached _asniagara_system (Variables|Character|GetMesh) "None" "0, 0, 0" "0, 0, 0" "KeepRelativeOffset" true))
        (bind _returnvalue_4 (Rendering|Material|CreateDynamicMaterialInstance _mesh 0 (Rendering|Material|GetMaterial _mesh 0) "None" :!class /Script/Engine.PrimitiveComponent))
        (bind _returnvalue_5 (Rendering|Material|GetVectorParameterValue _returnvalue_4 "DissolveEdgeColor" :!class /Script/Engine.MaterialInstanceDynamic))
        (Niagara|SetNiagaraVariable(LinearColor) _returnvalue_3 "DissolveParticleColor" _returnvalue_5)
        (Components|Timeline|SetPlayRate (Variables|Default|GetDissolveTimeline) (/ 1.0 (Variables|Default|GetTotalDissolveTime)))
        (bind _normalizedfloattrack (Timeline|DissolveTimeline PlayFromStart)
          (:Update
            (Rendering|Material|SetScalarParameterValueonMaterials (Variables|Character|GetMesh) "DissolveAmount" _normalizedfloattrack)
            (Utilities|IsValid _returnvalue_2
              (:Is%20Valid
                (Rendering|Material|SetScalarParameterValueonMaterials (Variables|/Script/PanWolfWar.PanWarWeaponBase|GetWeaponMesh _returnvalue_2) "DissolveAmount" _normalizedfloattrack)
                (if (and (> _normalizedfloattrack 0.5) (not (Variables|Default|GetTriedToSpawnStone?)))
                  (Variables|Default|SetTriedToSpawnStone? true)
                  (bind (_isstonetospawn_ _spawnlocation) (CallFunction|TrySpawnStone))
                  (if _isstonetospawn_
                    (|SpawnStone _spawnlocation))))))
          (:Finished
            (Utilities|IsValid _returnvalue
              (:Is%20Valid
                (Actor|DestroyActor _returnvalue))
              (:Is%20Not%20Valid
                _))
            (Actor|DestroyActor)))))))

(fn ConstructionScript)

(fn TrySpawnStone
  (bind _returnvalue (Transformation|GetActorLocation))
  (Utilities|FlowControl|Sequence
    (:then_0
      (bind (_outhit _returnvalue_2) (Collision|LineTraceForObjects _returnvalue (+ _returnvalue (* (Transformation|GetActorUpVector) -2e+02)) (Utilities|Array|MakeArray "ObjectTypeQuery1") false 0 "None"))
      (if _returnvalue_2
        (bind _randomlocation (Class|NavigationSystemV1|GetRandomLocationinNavigableRadius (.ImpactPoint (Collision|BreakHitResult _outhit)) 2e+02 0 0))
        (LocalVariables|SetRandomSpawnStoneLocation _randomlocation)))
    (:then_1
      (if (Math|Random|RandomBoolwithWeight 0.5)
        (Variables|Default|SetStoneClassToSpawn "/Game/Interactable/PickUps/BP_HealingStone.BP_HealingStone_C")
        (else
          (Variables|Default|SetStoneClassToSpawn "/Game/Interactable/PickUps/BP_HealingStone.BP_HealingStone_C")))
      (if (Math|Random|RandomBoolwithWeight (Class|EnemyAttributeComponent|GetStoneSpawnProbability (Variables|Default|GetEnemyAttributeComponent)))
        (return true (LocalVariables|GetRandomSpawnStoneLocation))
        (else
          (return false "0, 0, 0"))))))

(fn SpawnWeapon
  (bind _self self)
  (bind _returnvalue (Game|SpawnActorfromClass (Variables|Weapon|GetWeaponClassToSpawn) (Math|Transform|MakeTransform "0, 0, 0" "0, 0, 0" "1.000000,1.000000,1.000000") "AdjustIfPossibleButAlwaysSpawn" "MultiplyWithRoot" _self _self))
  (Utilities|IsValid _returnvalue
    (:Is%20Valid
      (Transformation|AttachComponentToComponent _returnvalue (Variables|Character|GetMesh) (Variables|Weapon|GetWeaponSocketNameToAttachTo) "SnapToTarget" "KeepRelative" "KeepWorld" true)
      (Class|PawnCombatComponent|EquipWeapon (Variables|Default|GetEnemyCombatComponent) _returnvalue)
      (Rendering|Material|SetScalarParameterValueonMaterials (Variables|/Script/PanWolfWar.PanWarWeaponBase|GetWeaponMesh _returnvalue) "DissolveAmount" 1.0))))