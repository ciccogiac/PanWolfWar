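; Base boss character that handles entrance presentation, boss health bar, and death sequence.
; On spawn it reverses a dissolve timeline, plays a random entry montage and registers the bar with EnemyUIComponent.
; On death it async-loads a Niagara effect tinted from the material's edge color and dissolves the mesh before destruction.
; Halfway through, it spawns a healing stone near a navigable ground point, ignoring the placement check's success flag.
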(event EventBeginPlay
  (bind _entrymontagestoplay (Variables|Default|GetEntryMontagesToPlay))
  (Utilities|FlowControl|Sequence
    (:then_0
      (Components|Timeline|SetPlayRate (Variables|Default|GetEntryRestoreTimeline) (/ 1.0 (Variables|Default|GetTotalEntryRestoreTime)))
      (bind _normalizedfloattrack (Timeline|EntryRestoreTimeline ReverseFromEnd)
        (:Update
          (Rendering|Material|SetScalarParameterValueonMaterials (Variables|Character|GetMesh) "DissolveAmount" _normalizedfloattrack))))
    (:then_1
      (if (Utilities|Array|IsNotEmpty _entrymontagestoplay)
        (Animation|PlayAnimMontage (.OutItem (Utilities|Array|Random _entrymontagestoplay)) 1.0 "None")))
    (:then_2
      (CallFunction|DrawBossBar))))

(event EventOnEnemyDieEvent
  (bind _mesh (Variables|Character|GetMesh))
  (bind _dissolveniagarasystem (Variables|Default|GetDissolveNiagaraSystem))
  (if (Utilities|IsValidSoftObjectReference _dissolveniagarasystem)
    (bind _object (Utilities|AsyncLoadAsset _dissolveniagarasystem)
      (:Completed
        (bind _asniagara_system (Utilities|Casting|CastToNiagaraSystem _object))
        (bind _returnvalue (Niagara|SpawnSystemAttached _asniagara_system (Variables|Character|GetMesh) "None" "0, 0, 0" "0, 0, 0" "KeepRelativeOffset" true))
        (bind _returnvalue_2 (Rendering|Material|CreateDynamicMaterialInstance _mesh 0 (Rendering|Material|GetMaterial _mesh 0) "None" :!class /Script/Engine.PrimitiveComponent))
        (bind _returnvalue_3 (Rendering|Material|GetVectorParameterValue _returnvalue_2 "DissolveEdgeColor" :!class /Script/Engine.MaterialInstanceDynamic))
        (Niagara|SetNiagaraVariable(LinearColor) _returnvalue "DissolveParticleColor" _returnvalue_3)
        (Components|Timeline|SetPlayRate (Variables|Default|GetDissolveTimeline) (/ 1.0 (Variables|Default|GetTotalDissolveTime)))
        (bind _normalizedfloattrack (Timeline|DissolveTimeline PlayFromStart)
          (:Update
            (Rendering|Material|SetScalarParameterValueonMaterials (Variables|Character|GetMesh) "DissolveAmount" _normalizedfloattrack)
            (if (and (> _normalizedfloattrack 0.5) (not (Variables|Default|GetTriedToSpawnStone?)))
              (Variables|Default|SetTriedToSpawnStone? true)
              (bind _spawnlocation (CallFunction|TrySpawnStone))
              (if true
                (|SpawnStone _spawnlocation))))
          (:Finished
            (Actor|DestroyActor)))))))

(fn ConstructionScript)

(fn DrawBossBar
  (bind _returnvalue (UserInterface|CreateWidget "/Game/UI/Widgets/EnemyWidgets/WBP_DefaultBossHealthBar.WBP_DefaultBossHealthBar_C"))
  (Rendering|Components|TextRender|SetText (Variables|/Game/UI/Widgets/EnemyWidgets/WBP_DefaultBossHealthBar.WBP_DefaultBossHealthBar_C|GetTextBlock_BossNameText _returnvalue) (Variables|Default|GetBossName))
  (UserInterface|Viewport|AddtoViewport _returnvalue 0)
  (Class|PanWarWidgetBase|InitEnemyCreatedWidget _returnvalue self)
  (Class|EnemyUIComponent|RegisterEnemyDrawnWidget (Variables|Default|GetEnemyUIComponent) _returnvalue))

(fn TrySpawnStone
  (bind _returnvalue (Transformation|GetActorLocation))
  (Utilities|FlowControl|Sequence
    (:then_0
      (bind (_outhit _returnvalue_2) (Collision|LineTraceForObjects _returnvalue (+ _returnvalue (* (Transformation|GetActorUpVector) -2e+02)) (Utilities|Array|MakeArray "ObjectTypeQuery1") false 0 "None"))
      (if _returnvalue_2
        (bind _randomlocation (Class|NavigationSystemV1|GetRandomLocationinNavigableRadius (.ImpactPoint (Collision|BreakHitResult _outhit)) 1e+02 0 0))
        (LocalVariables|SetRandomSpawnStoneLocation _randomlocation)
        (else
          (return false "0, 0, 0"))))
    (:then_1
      (if (Math|Random|RandomBoolwithWeight 0.5)
        (Variables|Default|SetStoneClassToSpawn "/Game/Interactable/PickUps/BP_HealingStone.BP_HealingStone_C")
        (else
          (Variables|Default|SetStoneClassToSpawn "/Game/Interactable/PickUps/BP_HealingStone.BP_HealingStone_C")))
      (return true (LocalVariables|GetRandomSpawnStoneLocation)))))