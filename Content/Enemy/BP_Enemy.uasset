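; BP_Enemy is an enemy that the third-person player can assassinate from a trigger box.
; While the player overlaps Box_Assassination, it shows a prompt widget and registers itself on the player as the stealth target.
; Assassinated plays a death montage, marks it dead and disables the box.
; The montage notify triggers ragdoll, Niagara effect and camera shake; completion removes capsule collision and destroys the actor after a short delay.
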(event OnComponentBeginOverlap(Box_Assassination)
  (params (OverlappedComponent :type Primitive%20Component%20Object%20Reference) (OtherActor :type Actor%20Object%20Reference) (OtherComp :type Primitive%20Component%20Object%20Reference) (OtherBodyIndex :type Integer) (bFromSweep :type Boolean) (SweepResult :type Hit%20Result%20Structure%20%28by%20ref%29))
  (bind _charref (Variables|Default|GetCharRef))
  (if (and (== _charref OtherActor) (not (Variables|Default|GetDie)))
    (Development|PrintString "Hello")
    (Variables|/Game/ThirdPerson/Blueprints/BP_ThirdPersonCharacter.BP_ThirdPersonCharacter_C|SetCanStealth _charref true)
    (Variables|/Game/ThirdPerson/Blueprints/BP_ThirdPersonCharacter.BP_ThirdPersonCharacter_C|SetEnemy_Assassin _charref self)
    (Rendering|SetVisibility (Variables|Default|GetAssassinate_Widget) true false)))

(event OnComponentEndOverlap(Box_Assassination)
  (params (OverlappedComponent :type Primitive%20Component%20Object%20Reference) (OtherActor :type Actor%20Object%20Reference) (OtherComp :type Primitive%20Component%20Object%20Reference) (OtherBodyIndex :type Integer))
  (bind _charref (Variables|Default|GetCharRef))
  (if (and (== _charref OtherActor) (not (Variables|Default|GetDie)))
    (Development|PrintString "By")
    (Variables|/Game/ThirdPerson/Blueprints/BP_ThirdPersonCharacter.BP_ThirdPersonCharacter_C|SetCanStealth _charref false)
    (Variables|/Game/ThirdPerson/Blueprints/BP_ThirdPersonCharacter.BP_ThirdPersonCharacter_C|SetEnemy_Assassin _charref 0)
    (Rendering|SetVisibility (Variables|Default|GetAssassinate_Widget) false false)))

(event Custom|Assassinated
  (Animation|Montage|PlayMontage (Variables|Character|GetMesh) "/Game/Enemy/Assassination/Assassination3_Die_AS_Montage.Assassination3_Die_AS_Montage"
    (:then
      (Variables|Default|SetDie true)
      (Rendering|SetVisibility (Variables|Default|GetAssassinate_Widget) false false)
      (Collision|SetCollisionEnabled (Variables|Default|GetBox_Assassination) "NoCollision"))
    (:OnCompleted
      (Collision|SetCollisionEnabled (Variables|Collision|GetCapsuleComponent) "NoCollision")
      (Utilities|FlowControl|Delay 0.7)
      (Actor|DestroyActor))
    (:OnNotifyBegin
      (Components|Activation|SetActive (Variables|Default|GetNiagara) true false)
      (Physics|SetSimulatePhysics (Variables|Character|GetMesh) true)
      (Camera|PlayWorldCameraShake "/Game/Enemy/Assassination/Hit_Shake.Hit_Shake_C" (Transformation|GetActorLocation) 4444.0 4444.0))))

(event EventBeginPlay
  (bind _asbp_third_person_character (Utilities|Casting|CastToBP_ThirdPersonCharacter (Game|GetPlayerCharacter 0)))
  (Variables|Default|SetCharRef _asbp_third_person_character)
  (Rendering|SetVisibility (Variables|Default|GetSkeletalMesh_Attacker) false false))

(fn ConstructionScript)